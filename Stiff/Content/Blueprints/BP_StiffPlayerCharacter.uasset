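; First-person player character that walks, looks, jumps and fires a gun through Enhanced Input, with the IM_Stiff mapping context added on possession.
; BeginPlay creates the gun as a child actor component snapped to the GripPoint socket on 1PMesh.
; Movement follows control yaw only.
; Each fire press calls Fire on the BP_EntGun child, rate-limited by the EnableFire flag that a ShootingDelay timer resets.
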(event `self.ReceiveBeginPlay`
  (bind _returnvalue (`AddComponent|NODE_AddChildActorComponent-0`))
  (bind _output_get (set `self.Gun` _returnvalue))
  (`SceneComponent.K2_AttachToComponent` _output_get (`self.1PMesh`) "GripPoint" "SnapToTarget" "SnapToTarget" "SnapToTarget" true))

(event `self.ReceivePossessed`
  (params (NewController :type "Controller Object Reference"))
  (bind _asplayer_controller (cast `PlayerController` NewController))
  (`EnhancedInputSubsystemInterface.AddMappingContext` (pcsubsystem `EnhancedInputLocalPlayerSubsystem` _asplayer_controller) "/Game/Input/IM_Stiff.IM_Stiff" 0 (struct)))

(event `EnhancedInput|/Game/Input/IA_MoveForwardStiff`
  (params (ActionValue :type "Float (double-precision)") (ElapsedSeconds :type "Float (double-precision)") (TriggeredSeconds :type "Float (double-precision)") (InputAction :type "InputAction Object Reference" :default "/Game/Input/IA_MoveForwardStiff.IA_MoveForwardStiff"))
  (:`Triggered`
    (`self.AddMovementInput` (`KismetMathLibrary.GetForwardVector` (`KismetMathLibrary.MakeRotator` 0.0 0.0 (.yaw (`self.GetControlRotation`)))) ActionValue)))

(event `EnhancedInput|/Game/Input/IA_MoveRightStiff`
  (params (ActionValue :type "Float (double-precision)") (ElapsedSeconds :type "Float (double-precision)") (TriggeredSeconds :type "Float (double-precision)") (InputAction :type "InputAction Object Reference" :default "/Game/Input/IA_MoveRightStiff.IA_MoveRightStiff"))
  (:`Triggered`
    (`self.AddMovementInput` (`KismetMathLibrary.GetRightVector` (`KismetMathLibrary.MakeRotator` 0.0 0.0 (.yaw (`self.GetControlRotation`)))) ActionValue)))

(event `EnhancedInput|/Game/Input/IA_LookStiff`
  (params (ActionValue :type "Vector2D Structure") (ElapsedSeconds :type "Float (double-precision)") (TriggeredSeconds :type "Float (double-precision)") (InputAction :type "InputAction Object Reference" :default "/Game/Input/IA_LookStiff.IA_LookStiff"))
  (:`Triggered`
    (`self.AddControllerYawInput` ActionValue_X)
    (`self.AddControllerPitchInput` ActionValue_Y)))

(event `EnhancedInput|/Game/Input/IA_JumpStiff`
  (params (ActionValue :type Boolean) (ElapsedSeconds :type "Float (double-precision)") (TriggeredSeconds :type "Float (double-precision)") (InputAction :type "InputAction Object Reference" :default "/Game/Input/IA_JumpStiff.IA_JumpStiff"))
  (:`Started`
    (`self.Jump`))
  (:`Completed`
    (`self.StopJumping`)))

(event `EnhancedInput|/Game/Input/IA_FireStiff`
  (params (ActionValue :type Boolean) (ElapsedSeconds :type "Float (double-precision)") (TriggeredSeconds :type "Float (double-precision)") (InputAction :type "InputAction Object Reference" :default "/Game/Input/IA_FireStiff.IA_FireStiff"))
  (:`Started`
    (if (`self.EnableFire`)
      (set `self.EnableFire` false)
      (bind _asbp_ent_gun (cast `/Game/Blueprints/BP_EntGun` (`ChildActorComponent.ChildActor` (`self.Gun`))))
      (`/Game/Blueprints/BP_EntGun.Fire` _asbp_ent_gun)
      (`KismetSystemLibrary.K2_SetTimer` null "SetEnableFire" (`self.ShootingDelay`)))))

(fn `SetEnableFire`
  (set `self.EnableFire` true))

(fn `UserConstructionScript`)